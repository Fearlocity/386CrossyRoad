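; Player character for a Crossy Road-style hopping game, with a score, a HUD and game-over handling.
; Movement input box-traces ahead, then launches the character in a short hop on a half-second cooldown while timelines turn the mesh toward the hop direction.
; Water and Hitbycar events show the GameOver widget and disable input, with a car hit also flattening the mesh.
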(event `InputAxis|MoveForward`
  (params (AxisValue :type "Float (single-precision)"))
  (bind _returnvalue (`self.K2_GetActorLocation`))
  (bind _staticmesh (`self.StaticMesh`))
  (bind _staticmesh_2 (`self.StaticMesh`))
  (if (and (> (`KismetMathLibrary.Abs` AxisValue) 0.3) (`self.CanMove`))
    (bind (_outhit _returnvalue_2) (`KismetSystemLibrary.BoxTraceSingle` _returnvalue (+ _returnvalue (* (`KismetMathLibrary.GetForwardVector` (`self.K2_GetActorRotation`)) (* (100.0 0.0 0.0) AxisValue))) (20.0 20.0 20.0) (struct) "TraceTypeQuery1"))
    (if (not _returnvalue_2)
      (`self.MoveCooldown`)
      (`self.LaunchCharacter` (`KismetMathLibrary.MakeVector` (* AxisValue 200.0) 0.0 200.0) true true)
      (if (> AxisValue 0.3)
        (bind (_direction _newtrack_0) (`Timeline|Timeline` :!via `PlayFromStart`)
          (:`Update`
            (`SceneComponent.K2_SetWorldRotation` _staticmesh (`KismetMathLibrary.RLerp` (`SceneComponent.K2_GetComponentRotation` _staticmesh) (struct :`Yaw` -90.0) _newtrack_0 true) false false)))
        (else
          (bind (_direction_2 _newtrack_0_2) (`Timeline|Timeline_0` :!via `PlayFromStart`)
            (:`Update`
              (`SceneComponent.K2_SetWorldRotation` _staticmesh_2 (`KismetMathLibrary.RLerp` (`SceneComponent.K2_GetComponentRotation` _staticmesh_2) (struct :`Yaw` 90.0) _newtrack_0_2 true) false false))))))))

(event `InputAxis|MoveRight`
  (params (AxisValue :type "Float (single-precision)"))
  (bind _returnvalue (`self.K2_GetActorLocation`))
  (bind _staticmesh (`self.StaticMesh`))
  (bind _staticmesh_2 (`self.StaticMesh`))
  (if (and (> (`KismetMathLibrary.Abs` AxisValue) 0.3) (`self.CanMove`))
    (bind (_outhit _returnvalue_2) (`KismetSystemLibrary.BoxTraceSingle` _returnvalue (+ _returnvalue (* (`KismetMathLibrary.GetRightVector` (`self.K2_GetActorRotation`)) (* (0.0 100.0 0.0) AxisValue))) (20.0 20.0 20.0) (struct) "TraceTypeQuery1"))
    (if (not _returnvalue_2)
      (`self.MoveCooldown`)
      (`self.LaunchCharacter` (`KismetMathLibrary.MakeVector` 0.0 (* AxisValue 200.0) 200.0) true true)
      (if (> AxisValue 0.3)
        (bind (_direction _newtrack_0) (`Timeline|Timeline_1` :!via `PlayFromStart`)
          (:`Update`
            (`SceneComponent.K2_SetWorldRotation` _staticmesh_2 (`KismetMathLibrary.RLerp` (`SceneComponent.K2_GetComponentRotation` _staticmesh_2) (struct) _newtrack_0 true) false false)))
        (else
          (bind (_direction_2 _newtrack_0_2) (`Timeline|Timeline_2` :!via `PlayFromStart`)
            (:`Update`
              (`SceneComponent.K2_SetWorldRotation` _staticmesh (`KismetMathLibrary.RLerp` (`SceneComponent.K2_GetComponentRotation` _staticmesh) (struct :`Yaw` -180.0) _newtrack_0_2 true) false false))))))))

(event `MoveCooldown`
  (`/Engine/EditorBlueprintResources/StandardMacros.DoOnce` false :!label _label
    (:`Completed`
      (set `self.CanMove` false)
      (`KismetSystemLibrary.Delay` 0.5)
      (set `self.CanMove` true)
      (goto _label :!via `Reset`))))

(event `Water`
  (bind _returnvalue (`|CreateWidget` "/Game/Characters/GameOver.GameOver_C" :!label _label_2))
  (`UserWidget.AddToViewport` _returnvalue 0)
  (set `PlayerController.bShowMouseCursor` true (`GameplayStatics.GetPlayerController` 0))
  (`self.DisableInput` (`GameplayStatics.GetPlayerController` 0)))

(event `Hitbycar`
  (`SceneComponent.SetWorldScale3D` (`self.StaticMesh`) (0.5 0.5 0.1))
  (goto _label_2))

(event `UpdateScore`
  (bind _result (`/Engine/EditorBlueprintResources/StandardMacros.IncrementFloat` (`self.Score`))
    (:`  `
      (set `self.Score` _result))))

(event `self.ReceiveBeginPlay`
  (bind _returnvalue (`|CreateWidget` "/Game/Characters/HUD.HUD_C"))
  (`UserWidget.AddToViewport` _returnvalue 0))

(fn `UserConstructionScript`
  (`parent.UserConstructionScript`))
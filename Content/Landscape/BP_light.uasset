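; BP_light is a landscape light actor that flashes alternately between one blue light and two red lights.
; Tick runs through a one-second Delay, which throttles the switching to roughly once per second.
; A Seconds variable serves as the toggle: at zero it lights blue and sets the counter to three, otherwise it lights both reds and subtracts three.
; Switching works by setting each light's intensity to full or zero.
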(event `self.ReceiveTick`
  (params (DeltaSeconds :type "Float (single-precision)"))
  (`KismetSystemLibrary.Delay` 1.0)
  (if (== (`self.Seconds`) 0)
    (`LightComponent.SetIntensity` (`self.Bluelight`) 25000.0)
    (`LightComponent.SetIntensity` (`self.Redlight1`) 0.0)
    (`LightComponent.SetIntensity` (`self.Redlight`) 0.0)
    (set `self.Seconds` 3)
    (else
      (`LightComponent.SetIntensity` (`self.Redlight`) 25000.0)
      (`LightComponent.SetIntensity` (`self.Redlight1`) 25000.0)
      (`LightComponent.SetIntensity` (`self.Bluelight`) 0.0)
      (set `self.Seconds` (- (`self.Seconds`) 3)))))

(fn `UserConstructionScript`)